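; A test interactable actor Blueprint that prints a placeholder message when interacted with.
; When ShowDebugName is on and the actor was recently rendered, Tick rotates the DebugName component to face the player camera, billboarding the label.
; BeginPlay, overlap and the construction script are empty.
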(event EventBeginPlay)

(event Collision|EventActorBeginOverlap
  (params (OtherActor :type Actor%20Object%20Reference)))

(event EventTick
  (params (DeltaSeconds :type Float%20%28single-precision%29))
  (bind _debugname (Variables|Default|GetDebugName))
  (if (and (Variables|Default|GetbShowDebugName) (Class|Actor|WasRecentlyRendered 0.2))
    (Transformation|SetWorldRotation _debugname (Math|Rotator|FindLookatRotation (Transformation|GetWorldLocation _debugname) (Camera|GetCameraLocation (Game|GetPlayerCameraManager 0))) false false)))

(event EventOnInteract
  (Development|PrintString "Stuff!"))

(fn ConstructionScript)