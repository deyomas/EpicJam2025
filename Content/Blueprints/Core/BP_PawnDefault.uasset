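; Default pawn that handles crouching and interaction, with Move, Jump and Look events left as empty stubs.
; Each tick, a debug-drawn box trace from the camera finds BPI_Interactable actors, moving the highlight to new targets and clearing it when nothing is hit.
; Interact messages the stored target.
; Crouch switches capsule half-height, while the construction script scales the Cube's height to match the capsule.
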(event EventTick
  (params (DeltaSeconds :type Float%20%28single-precision%29))
  (CallFunction|CastforInteractable))

(event EventJump
  (params (bJumpPressed :type Boolean))
  ;[0.15 0.15 0.15 0.5] Movement
)

(event EventMove
  (params (movement :type Vector%20%28by%20ref%29 :default "0, 0, 0"))
  ;[0.15 0.15 0.15 0.5] Movement
)

(event EventInteract
  ;[0.15 0.15 0.15 0.5] Movement
  (bind _availableinteractable (Variables|Default|GetAvailableInteractable)
    (:then
      (Class|BPIInteractable|OnInteract(Message) _availableinteractable))
    (:else)))

(event EventCrouch
  (params (bCrouched :type Boolean))
  ;[0.15 0.15 0.15 0.5] Movement
  (Development|PrintString (Utilities|String|ToString(Boolean) bCrouched))
  (Components|Capsule|SetCapsuleHalfHeight (Variables|Default|GetCapsule) (Math|Float|SelectFloat 22.0 44.0 bCrouched) true))

(event EventLook
  (params (Value :type Vector%202D%20Structure%20%28by%20ref%29))
  ;[0.15 0.15 0.15 0.5] Movement
)

(fn ConstructionScript
  (bind _cube (Variables|Default|GetCube))
  (bind _relativescale3d (Variables|/Script/Engine.SceneComponent|GetRelativeScale3D _cube))
  (Transformation|SetRelativeScale3D _cube (Math|Vector|MakeVector (.x _relativescale3d) (.y _relativescale3d) (* (Variables|/Script/Engine.CapsuleComponent|GetCapsuleHalfHeight (Variables|Default|GetCapsule)) 2.0 0.01))))

(fn CastforInteractable
  (bind _camera (Variables|Default|GetCamera))
  (bind _camera_2 (Variables|Default|GetCamera))
  (bind _returnvalue (Transformation|GetWorldLocation _camera))
  (bind (_outhit _returnvalue_2) (Collision|BoxTraceByChannel _returnvalue (+ _returnvalue (* (Math|Vector|GetForwardVector _camera_2) (Variables|Default|GetInteractableTraceDistance))) (Math|Conversions|ToVector(Float) (Variables|Default|GetInteractableTraceSize)) (Transformation|GetWorldRotation _camera_2) "TraceTypeQuery3" false 0 "ForOneFrame"))
  (if _returnvalue_2
    (if (Utilities|DoesObjectImplementInterface (.HitActor (Collision|BreakHitResult _outhit)) "/Game/Blueprints/Interactable/BPI_Interactable.BPI_Interactable_C")
      (if (!= (Variables|Default|GetAvailableInteractable) (.HitActor (Collision|BreakHitResult _outhit)))
        (Utilities|FlowControl|Sequence
          (:then_0
            (bind _availableinteractable (Variables|Default|GetAvailableInteractable)
              (:then
                (Class|BPIInteractable|SetHighlight(Message) _availableinteractable false))
              (:else)))
          (:then_1
            (bind _output_get (Variables|Default|SetAvailableInteractable (.HitActor (Collision|BreakHitResult _outhit))))
            (Class|BPIInteractable|SetHighlight(Message) _output_get true)))))
    (else
      (bind _availableinteractable_2 (Variables|Default|GetAvailableInteractable)
        (:then
          (Class|BPIInteractable|SetHighlight(Message) _availableinteractable_2 false)
          (Variables|Default|SetAvailableInteractable 0))
        (:else)))))